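; Actor component for character abilities that holds the owner's active abilities and hotbar layouts.
; On initialization it spawns a melee ability actor at the owner's transform, registers it as active, and binds a test dispatcher that executes it on the stored targets.
; A temporary setup function fills every hotbar slot with that melee ability, and getters expose the hotbars.
; ExecAbilityInSlot is a stub that only returns the buttons-per-hotbar value.
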(event Custom|TestInit
  (Class|ILCAbility|ExecuteAbility(Message) (Variables|Default|GetMelee%20Parent) (Components|GetOwner) (Variables|Default|GetTargets)))

(event EventTick
  (params (DeltaSeconds :type Float%20%28single-precision%29)))

(event EventInitializeComponent
  (bind _returnvalue (Components|GetOwner))
  (EventDispatchers|BindEventtoTestInitDispatcher (delegate Custom|TestInit))
  (Variables|Default|SetOwner _returnvalue)
  (bind _returnvalue_2 (Game|SpawnActorfromClass "/Game/Blueprints/Logic_Classes/Abilities/Abilities_Melee/LC_Ability_Melee_Parent.LC_Ability_Melee_Parent_C" (Transformation|GetActorTransform _returnvalue) true 0))
  (bind _output_get (Variables|Default|SetMelee%20Parent _returnvalue_2))
  (Utilities|Array|AddUnique (Variables|Core|GetActiveAbililities) _output_get))

(fn TempHotBarSetup
  (bind _melee_parent (Variables|Default|GetMelee%20Parent))
  (for _index (range 0 (- (Utilities|Array|Length (Variables|UILoaders|GetHotBars)) 1))
    (bind _output_get (LocalVariables|SetTest (Utilities|Struct|MakeStruct_HotBarAbilities _melee_parent _melee_parent _melee_parent _melee_parent _melee_parent)))
    (Utilities|Array|SetArrayElem (Variables|UILoaders|GetHotBars) _index _output_get true)))

(fn ExecAbilityinSlot
  (return (Variables|UILoaders|GetButtonsPerHotbar)))

(fn GetAllHotbars
  (return (Variables|UILoaders|GetHotBars)))

(fn GetHotbarbyIndex
  (params (Hotbar%20Index :type Integer))
  (return (Utilities|Array|Get(acopy) (Variables|UILoaders|GetHotBars) Hotbar%20Index)))