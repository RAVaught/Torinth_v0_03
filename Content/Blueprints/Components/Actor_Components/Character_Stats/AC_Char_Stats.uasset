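; Actor component that holds a character's stats, with experience, derived tuning values and getters for values, structs and waves.
; Add and subtract experience events apply each stat's modifier and range-check against its level threshold before writing back to StatBlock.
; Helper functions derive amplitude, frequency and experience-to-level from summed stats, and compute sine-based wave values around each level.
; Wave-parameter increment and decrement events are empty stubs.
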(event EventTick
  (params (DeltaSeconds :type Float%20%28single-precision%29)))

(event EventInitializeComponent)

(event EventAddExperience
  (params (Stat :type EC_Char_Stats%20Enum :default "NewEnumerator0") (Amount :type Integer))
  ;[1 1 1] Contains all Interface Functions that do not return a value (because they don't sshow up in the interface list.)
  (bind _stat_struct (Components|AC|CharStats|Private|GetStatStruct Stat))
  (bind _case (CallFunction|IntBetweentoInt (Math|Float|Floor (|(amount*expMod)+amount+curExp (Math|Conversions|ToFloat(Integer) (.CurrentExperience (Utilities|Struct|BreakStruct_Char_Stats _stat_struct))) (.ExperienceModifier (Utilities|Struct|BreakStruct_Char_Stats _stat_struct)) (Math|Conversions|ToFloat(Integer) (+ Amount (.CurrentExperience (Utilities|Struct|BreakStruct_Char_Stats _stat_struct)))))) (Variables|Default|GettIntZero) (.ExpToLevel (Utilities|Struct|BreakStruct_Char_Stats _stat_struct))))
  (switch int _case
    (:0
      (Utilities|Struct|SetmembersinStruct_Char_Stats _stat_struct (Math|Float|Floor (|(amount*expMod)+amount+curExp (Math|Conversions|ToFloat(Integer) (.CurrentExperience (Utilities|Struct|BreakStruct_Char_Stats _stat_struct))) (.ExperienceModifier (Utilities|Struct|BreakStruct_Char_Stats _stat_struct)) (Math|Conversions|ToFloat(Integer) (+ Amount (.CurrentExperience (Utilities|Struct|BreakStruct_Char_Stats _stat_struct)))))))
      (Utilities|Array|SetArrayElem (Variables|Components|AC_Char_Stats|CoreData|GetStatBlock) (Math|Conversions|ToInteger(Byte) Stat) _stat_struct))))

(event EventSubtractExperience
  (params (Stat :type EC_Char_Stats%20Enum :default "NewEnumerator0") (Amount :type Integer))
  ;[1 1 1] Contains all Interface Functions that do not return a value (because they don't sshow up in the interface list.)
  (bind _stat_struct (Components|AC|CharStats|Private|GetStatStruct Stat))
  (bind _case (CallFunction|IntBetweentoInt (Math|Float|Floor (|curExp-(amount-(amount*expMod)) (Math|Conversions|ToFloat(Integer) (.CurrentExperience (Utilities|Struct|BreakStruct_Char_Stats _stat_struct))) (Math|Conversions|ToFloat(Integer) Amount) (.ExperienceModifier (Utilities|Struct|BreakStruct_Char_Stats _stat_struct)))) (Variables|Default|GettIntZero) (.ExpToLevel (Utilities|Struct|BreakStruct_Char_Stats _stat_struct))))
  (switch int _case
    (:Default
      (Class|VisualLoggerKismetLibrary|LogText "AC_Char_Stats>Event Subtract Experience: Exception error: Can not determine value in range." "Component Log"))
    (:0
      (Utilities|Struct|SetmembersinStruct_Char_Stats _stat_struct (Math|Float|Floor (|curExp-(amount-(amount*expMod)) (Math|Conversions|ToFloat(Integer) (.CurrentExperience (Utilities|Struct|BreakStruct_Char_Stats _stat_struct))) (Math|Conversions|ToFloat(Integer) Amount) (.ExperienceModifier (Utilities|Struct|BreakStruct_Char_Stats _stat_struct)))))
      (Utilities|Array|SetArrayElem (Variables|Components|AC_Char_Stats|CoreData|GetStatBlock) (Math|Conversions|ToInteger(Byte) Stat) _stat_struct))))

(event EventDecrementAmplitude
  (params (Stat :type EC_Char_Stats%20Enum :default "NewEnumerator0") (Percentage :type Float%20%28single-precision%29))
  ;[1 1 1] Contains all Interface Functions that do not return a value (because they don't sshow up in the interface list.)
)

(event EventDecrementControl
  (params (Stat :type EC_Char_Stats%20Enum :default "NewEnumerator0"))
  ;[1 1 1] Contains all Interface Functions that do not return a value (because they don't sshow up in the interface list.)
)

(event EventDecrementFocus
  (params (Stat :type EC_Char_Stats%20Enum :default "NewEnumerator0"))
  ;[1 1 1] Contains all Interface Functions that do not return a value (because they don't sshow up in the interface list.)
)

(event EventDecrementFrequency
  (params (Stat :type EC_Char_Stats%20Enum :default "NewEnumerator0") (Percentage :type Float%20%28single-precision%29))
  ;[1 1 1] Contains all Interface Functions that do not return a value (because they don't sshow up in the interface list.)
)

(event EventDecrementPhase
  (params (Stat :type EC_Char_Stats%20Enum :default "NewEnumerator0") (Degrees :type Float%20%28single-precision%29))
  ;[1 1 1] Contains all Interface Functions that do not return a value (because they don't sshow up in the interface list.)
)

(event EventIncrementAmplitude
  (params (Stat :type EC_Char_Stats%20Enum :default "NewEnumerator0") (Percentage :type Float%20%28single-precision%29))
  ;[1 1 1] Contains all Interface Functions that do not return a value (because they don't sshow up in the interface list.)
)

(event EventIncrementControl
  (params (Stat :type EC_Char_Stats%20Enum :default "NewEnumerator0"))
  ;[1 1 1] Contains all Interface Functions that do not return a value (because they don't sshow up in the interface list.)
)

(event EventIncrementFocus
  (params (Stat :type EC_Char_Stats%20Enum :default "NewEnumerator0"))
  ;[1 1 1] Contains all Interface Functions that do not return a value (because they don't sshow up in the interface list.)
)

(event EventIncrementFrequency
  (params (Stat :type EC_Char_Stats%20Enum :default "NewEnumerator0") (Percentage :type Float%20%28single-precision%29))
  ;[1 1 1] Contains all Interface Functions that do not return a value (because they don't sshow up in the interface list.)
)

(event EventIncrementPhase
  (params (Stat :type EC_Char_Stats%20Enum :default "NewEnumerator0") (Degrees :type Float%20%28single-precision%29))
  ;[1 1 1] Contains all Interface Functions that do not return a value (because they don't sshow up in the interface list.)
)

(fn GetStatStruct
  (params (Stat :type EC_Char_Stats%20Enum :default "NewEnumerator0"))
  ;[1 1 1] Loops through the stat struct array. If a match is found, it breaks the loop and returns the struct.
  (bind _array_element (Utilities|Array|ForEachLoopwithBreak (Variables|Components|AC_Char_Stats|CoreData|GetStatBlock) :!label _label)
    (:LoopBody
      (if (Utilities|Enum|Equal(Enum) Stat (.StatID (Utilities|Struct|BreakStruct_Char_Stats _array_element)))
        (goto _label Break)))
    (:Completed
      (return _array_element))))

(fn CalculateStatWaves
  (for (_array_element _array_index) (Variables|Components|AC_Char_Stats|CoreData|GetStatBlock)
    (Utilities|Array|SetArrayElem (Variables|Components|AC_Char_Stats|CalculatedData|GetWaveValues) _array_index (|A*sin(freq*level+phase)+level (.Amplitude (Utilities|Struct|BreakStruct_Char_Stats _array_element)) (.Frequency (Utilities|Struct|BreakStruct_Char_Stats _array_element)) (Math|Conversions|ToFloat(Integer) (.CurrentValue (Utilities|Struct|BreakStruct_Char_Stats _array_element))) (.Phase (Utilities|Struct|BreakStruct_Char_Stats _array_element))) true)))

(fn CalculateAmplitude
  (params (Stat :type Struct%20Char%20Stats%20Structure%20%28by%20ref%29))
  (bind (_statid _currentvalue _maxvalue) (Utilities|Struct|BreakStruct_Char_Stats Stat))
  ;[1 1 1] Calculates the Amplitude as (SumOfAllLevels/(Maxvalue/CurValue))/ExpPercentToNextLevel
  (bind _sum (Components|AC|CharStats|Private|SumStats))
  (Utilities|Struct|SetmembersinStruct_Char_Stats Stat (|(sumOfLevels/(maxLevel-curLevel))/expPercentage (Math|Conversions|ToFloat(Integer) _maxvalue) (Math|Conversions|ToFloat(Integer) _currentvalue) (Math|Conversions|ToFloat(Integer) _sum) (Components|AC|CharStats|Private|CalculateExperiencePercentage Stat))))

(fn CalculateFrequency
  (params (Stat :type Struct%20Char%20Stats%20Structure%20%28by%20ref%29))
  (bind (_statid _currentvalue _maxvalue) (Utilities|Struct|BreakStruct_Char_Stats Stat))
  ;[1 1 1] Calculates the frequency of the stat using the formula:  (sumOfLevels/(maxLvl-curLvl))/expPercent
  (bind _sum (Components|AC|CharStats|Private|SumStats))
  (Utilities|Struct|SetmembersinStruct_Char_Stats Stat (|(sumOfLevels/(maxLvl-curLvl))/expPercent (Math|Conversions|ToFloat(Integer) _sum) (Math|Conversions|ToFloat(Integer) _maxvalue) (Math|Conversions|ToFloat(Integer) _currentvalue) (Components|AC|CharStats|Private|CalculateExperiencePercentage Stat))))

(fn SumStats
  ;[1 1 1] Reset prior to calculation.
  (LocalVariables|SetStatSum 0)
  ;[1 1 1] Gets the value for all stats and sums them, returning the sum.
  (for _array_element (Variables|Components|AC_Char_Stats|CalculatedData|GetStatValues)
    (LocalVariables|SetStatSum (+ _array_element (LocalVariables|GetStatSum))))
  (return (LocalVariables|GetStatSum)))

(fn CalculateExperiencetoLevel
  (params (Stat :type Struct%20Char%20Stats%20Structure%20%28by%20ref%29))
  (bind (_statid _currentvalue _maxvalue) (Utilities|Struct|BreakStruct_Char_Stats Stat))
  ;[1 1 1] EXP To Level = (lvl*5)(sum of all stats/(max level - current level))*max level
  (bind _sum (Components|AC|CharStats|Private|SumStats))
  (Utilities|Struct|SetmembersinStruct_Char_Stats Stat (Math|Float|Floor (|(curLevel*5)*(sumOfAllLevels/(maxLevel-curLevel))*(maxLevel) (Math|Conversions|ToFloat(Integer) _currentvalue) (Math|Conversions|ToFloat(Integer) _sum) (Math|Conversions|ToFloat(Integer) _maxvalue)))))

(fn CalculateStatPercentage
  (params (Stat :type Struct%20Char%20Stats%20Structure))
  (bind (_statid _currentvalue _maxvalue) (Utilities|Struct|BreakStruct_Char_Stats Stat))
  (return (/ (Math|Conversions|ToFloat(Integer) _currentvalue) (Math|Conversions|ToFloat(Integer) _maxvalue))))

(fn CalculateExperiencePercentage
  (params (Stat :type Struct%20Char%20Stats%20Structure%20%28by%20ref%29))
  (bind (_statid _currentvalue _maxvalue _currentexperience _exptolevel) (Utilities|Struct|BreakStruct_Char_Stats Stat))
  (return (/ (Math|Conversions|ToFloat(Integer) _currentexperience) (Math|Conversions|ToFloat(Integer) _exptolevel))))

(fn GetAllStats
  (return (Variables|Components|AC_Char_Stats|CalculatedData|GetStatValues)))

(fn GetAllStatWaves
  (return (Variables|Components|AC_Char_Stats|CalculatedData|GetWaveValues)))

(fn GetStat
  (params (Stat :type EC_Char_Stats%20Enum :default "NewEnumerator0"))
  (return (Utilities|Array|Get(acopy) (Variables|Components|AC_Char_Stats|CalculatedData|GetStatValues) (Math|Conversions|ToInteger(Byte) Stat))))

(fn GetStatInfo
  (params (StatToGet :type EC_Char_Stats%20Enum :default "NewEnumerator0"))
  (bind _stat_struct (Components|AC|CharStats|Private|GetStatStruct StatToGet))
  (return _stat_struct))

(fn GetStatWave
  (params (Stat :type EC_Char_Stats%20Enum :default "NewEnumerator0"))
  (return (Utilities|Array|Get(acopy) (Variables|Components|AC_Char_Stats|CalculatedData|GetWaveValues) (Math|Conversions|ToInteger(Byte) Stat))))